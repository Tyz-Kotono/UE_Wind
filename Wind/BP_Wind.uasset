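; BP_Wind is a wind actor that feeds the player's movement into Niagara and materials.
; On BeginPlay it caches the NPC_Wind parameter collection and third-person character, and passes the pawn to the NSGrid3DTest Niagara component.
; Each Tick it writes the player's foot position (actor location minus capsule half-height), previous position and velocity to the Niagara collection.
; It also mirrors the foot position to MPC_Wind for materials.
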(event EventBeginPlay
  (bind _returnvalue (Game|Player|GetPlayerPawn 0))
  (bind _returnvalue_2 (Class|NiagaraFunctionLibrary|GetNiagaraParameterCollection "/Game/Wind/NPC_Wind.NPC_Wind"))
  (Variables|Default|SetNPC_Wind _returnvalue_2)
  (Class|NiagaraComponent|SetVariableObject (Variables|Default|GetNS_Grid3DTest) "User.PlayerObject" _returnvalue)
  (bind _asbp_third_person_character (Utilities|Casting|CastToBP_ThirdPersonCharacter _returnvalue))
  (Variables|Default|SetThird%20Person%20Character _asbp_third_person_character))

(event Collision|EventActorBeginOverlap
  (params (OtherActor :type Actor%20Object%20Reference)))

(event EventTick
  (params (DeltaSeconds :type Float%20%28single-precision%29))
  (bind _returnvalue (Game|Player|GetPlayerPawn 0))
  (bind _npc_wind (Variables|Default|GetNPC_Wind))
  (Variables|Default|SetLocation (- (Transformation|GetActorLocation _returnvalue) (Math|Vector|MakeVector 0.0 0.0 (Components|Capsule|GetScaledCapsuleHalfHeight (Variables|/Script/Engine.Character|GetCapsuleComponent (Variables|Default|GetThird%20Person%20Character))))))
  (Effects|Components|ParticleSystem|SetVectorParameter _npc_wind "Position" (Variables|Default|GetLocation))
  (Effects|Components|ParticleSystem|SetVectorParameter _npc_wind "PrePosition" (Variables|Default|GetPreLocation))
  (Variables|Default|SetPreLocation (Variables|Default|GetLocation))
  (Effects|Components|ParticleSystem|SetVectorParameter (Variables|Default|GetNPC_Wind) "Velocity" (Transformation|GetVelocity _returnvalue))
  ;[0.15 0.15 0.15 0.5] Materials
  (Rendering|Material|SetVectorParameterValue "/Game/Wind/MPC_Wind.MPC_Wind" "Position" (Utilities|Struct|MakeLinearColor (.X (Math|Vector|BreakVector (Variables|Default|GetLocation))) (.Y (Math|Vector|BreakVector (Variables|Default|GetLocation))) (.Z (Math|Vector|BreakVector (Variables|Default|GetLocation))) 1.0) :!class /Script/Engine.KismetMaterialLibrary))

(fn ConstructionScript)